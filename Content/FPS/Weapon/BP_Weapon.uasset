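; FPS weapon Blueprint that plays cosmetic firing effects for a shot through its FireEffects event.
; It caches impact point, normal and surface type, selects the first- or third-person mesh outside dedicated servers, then reads the muzzle socket position.
; It lazily spawns and reuses three helper actors for fire (muzzle flash, tracer, shell eject), impacts and decals, passing each the impact data before calling Fire.
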(event EventFireEffects
  (params (ImpactPoint :type Vector%20%28by%20ref%29 :default "0, 0, 0") (ImpactNormal :type Vector%20%28by%20ref%29 :default "0, 0, 0") (ImpactSurfaceType :type EPhysicalSurface%20Enum :default "SurfaceType_Default") (bIsFirstPerson :type Boolean))
  (Utilities|FlowControl|Sequence
    (:then_0
      ;[0.15 0.15 0.15 0.5] Cache Initial Values
      (Variables|Default|SetIs%20First%20Person bIsFirstPerson)
      (if (not (Networking|IsDedicatedServer))
        (Variables|Default|SetImpact%20Points (Utilities|Array|MakeArray ImpactPoint))
        (Variables|Default|SetImpact%20Normal (Utilities|Array|MakeArray ImpactNormal))
        (Variables|Default|SetImpact%20Surface%20Type (Utilities|Array|MakeArray ImpactSurfaceType))
        ;[0.15 0.15 0.15 0.5] Cache Correct Mesh
        (if (Variables|Default|GetIs%20First%20Person)
          (Variables|Default|SetSkeletal%20Mesh (Variables|Default|GetMesh1P))
          (else
            (Variables|Default|SetSkeletal%20Mesh (Variables|Default|GetMesh3P))))))
    (:then_1
      ;[0.15 0.15 0.15 0.5] Cache Muzzle Position
      (Variables|Default|SetMuzzle%20Position (Transformation|GetSocketLocation (Variables|Default|GetSkeletal%20Mesh) (Variables|Default|GetMuzzle%20Socket%20Name))))
    (:then_2
      (Utilities|FlowControl|Sequence
        (:then_0
          (Utilities|IsValid (Variables|Default|GetWeapon%20Fire)
            (:Is%20Valid
              _)
            (:Is%20Not%20Valid
              ;[0.15 0.15 0.15 0.5] Weapon Fire
              (bind _returnvalue (Game|SpawnActorfromClass "/Game/Effects/Blueprints/B_WeaponFire.B_WeaponFire_C" (Math|Transform|MakeTransform "0, 0, 0") "Undefined" "MultiplyWithRoot" 0 (Variables|Default|GetSkeletal%20Mesh) true (Variables|Default|GetShell%20Eject%20System) true (Variables|Default|GetMuzzle%20Flash%20System) true (Variables|Default|GetTracer%20System) (Variables|Default|GetShell%20Eject%20Mesh) 0))
              (bind _output_get (Variables|Default|SetWeapon%20Fire _returnvalue))
              (Transformation|AttachComponentToComponent _output_get (Variables|Default|GetSkeletal%20Mesh) "None" "KeepRelative" "KeepRelative" "KeepRelative" true)))
          ;[0.15 0.15 0.15 0.5] Set Important values before calling fire
          (Variables|/Game/Effects/Blueprints/B_WeaponFire.B_WeaponFire_C|SetImpactPositions (Variables|Default|GetWeapon%20Fire) (Variables|Default|GetImpact%20Points))
          (Variables|/Game/Effects/Blueprints/B_WeaponFire.B_WeaponFire_C|SetImpactNormals (Variables|Default|GetWeapon%20Fire) (Variables|Default|GetImpact%20Normal))
          (Variables|/Game/Effects/Blueprints/B_WeaponFire.B_WeaponFire_C|SetImpactSurfaceTypes (Variables|Default|GetWeapon%20Fire) (Variables|Default|GetImpact%20Surface%20Type))
          ;[0.15 0.15 0.15 0.5] Actually fire the effect
          (Default|Fire (Variables|Default|GetWeapon%20Fire) (Variables|Default|GetIs%20First%20Person)))
        (:then_1
          (Utilities|IsValid (Variables|Default|GetWeapon%20Impacts)
            (:Is%20Valid
              _)
            (:Is%20Not%20Valid
              ;[0.15 0.15 0.15 0.5] Weapon Fire
              (bind _returnvalue_2 (Game|SpawnActorfromClass "/Game/Effects/Blueprints/B_WeaponImpacts.B_WeaponImpacts_C" (Math|Transform|MakeTransform "0, 0, 0") "Undefined" "MultiplyWithRoot" 0 5e+02 0))
              (bind _output_get_2 (Variables|Default|SetWeapon%20Impacts _returnvalue_2))
              (Transformation|AttachComponentToComponent _output_get_2 (Variables|Default|GetSkeletal%20Mesh) "None" "KeepRelative" "KeepRelative" "KeepRelative" true)))
          ;[0.15 0.15 0.15 0.5] Set Important values
          (Variables|/Game/Effects/Blueprints/B_WeaponImpacts.B_WeaponImpacts_C|SetImpactPositions (Variables|Default|GetWeapon%20Impacts) (Variables|Default|GetImpact%20Points))
          (Variables|/Game/Effects/Blueprints/B_WeaponImpacts.B_WeaponImpacts_C|SetImpactNormals (Variables|Default|GetWeapon%20Impacts) (Variables|Default|GetImpact%20Normal))
          (Variables|/Game/Effects/Blueprints/B_WeaponImpacts.B_WeaponImpacts_C|SetImpactSurfaceTypes (Variables|Default|GetWeapon%20Impacts) (Variables|Default|GetImpact%20Surface%20Type))
          (Variables|/Game/Effects/Blueprints/B_WeaponImpacts.B_WeaponImpacts_C|SetMuzzlePosition (Variables|Default|GetWeapon%20Impacts) (Variables|Default|GetMuzzle%20Position))
          ;[0.15 0.15 0.15 0.5] Actually Fire the Effect
          (Default|Fire (Variables|Default|GetWeapon%20Impacts) (Variables|Default|GetIs%20First%20Person)))
        (:then_2
          (Utilities|IsValid (Variables|Default|GetWeapon%20Decals)
            (:Is%20Valid
              _)
            (:Is%20Not%20Valid
              ;[0.15 0.15 0.15 0.5] Weapon Fire
              (bind _returnvalue_3 (Game|SpawnActorfromClass "/Game/Effects/Blueprints/B_WeaponDecals.B_WeaponDecals_C" (Math|Transform|MakeTransform "0, 0, 0") "Undefined" "MultiplyWithRoot" 0 0))
              (bind _output_get_3 (Variables|Default|SetWeapon%20Decals _returnvalue_3))
              (Transformation|AttachComponentToComponent _output_get_3 0 "None" "KeepRelative" "KeepRelative" "KeepRelative" true)))
          ;[0.15 0.15 0.15 0.5] Set Important Values
          (Variables|/Game/Effects/Blueprints/B_WeaponDecals.B_WeaponDecals_C|SetImpactPositions (Variables|Default|GetWeapon%20Decals) (Variables|Default|GetImpact%20Points))
          (Variables|/Game/Effects/Blueprints/B_WeaponDecals.B_WeaponDecals_C|SetImpactNormals (Variables|Default|GetWeapon%20Decals) (Variables|Default|GetImpact%20Normal))
          (Variables|/Game/Effects/Blueprints/B_WeaponDecals.B_WeaponDecals_C|SetImpact%20Surface%20Types (Variables|Default|GetWeapon%20Decals) (Variables|Default|GetImpact%20Surface%20Type))
          ;[0.15 0.15 0.15 0.5] Actually Fire the Effect
          (Default|Fire (Variables|Default|GetWeapon%20Decals) (Variables|Default|GetMuzzle%20Position)))))))

(fn ConstructionScript)
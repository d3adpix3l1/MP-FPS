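; Respawning ammo pickup that gives a weapon type's ammo to the actor overlapping its sphere.
; On overlap it hides the spinning mesh, plays a sound, deactivates collision, sends AddAmmoMessage to that actor and starts a respawn timer.
; Respawn restores visibility, rotation and collision through the IsActive flag and collision profile swaps, with a ready sound and Niagara effect.
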(event Custom|OnComponentBeginOverlap_Event
  (params (OverlappedComponent :type Primitive%20Component%20Object%20Reference) (OtherActor :type Actor%20Object%20Reference) (OtherComp :type Primitive%20Component%20Object%20Reference) (OtherBodyIndex :type Integer) (bFromSweep :type Boolean) (SweepResult :type Hit%20Result%20Structure%20%28by%20ref%29))
  (Variables|Default|SetOther%20Actor OtherActor)
  (Utilities|FlowControl|Sequence
    (:then_0
      ;[0.15 0.15 0.15 0.5] Hide mesh and play pickup sound
      (Rendering|SetVisibility (Variables|Default|GetSM_Weapon) false false)
      (Audio|PlaySoundatLocation (Variables|Default|GetPickup%20Sound) (Transformation|GetActorLocation) "0, 0, 0" 1.0 1.0 0.0 0 0 0 0))
    (:then_1
      ;[0.15 0.15 0.15 0.5] Disable sphere collision
      (Collision|SetCollisionProfileName (Variables|Default|GetSphere) (Variables|Default|GetInactive%20Collision%20Profile) true :!class /Script/Engine.PrimitiveComponent))
    (:then_2
      ;[0.15 0.15 0.15 0.5] Set Inactive
      (Variables|Default|SetIsActive false))
    (:then_3
      ;[0.15 0.15 0.15 0.5] Actually add ammo
      (Class|PlayerInterface|AddAmmo(Message) (Variables|Default|GetOther%20Actor) (Variables|Default|GetWeaponType) (Variables|Default|GetAmmo%20Amount)))
    (:then_4
      (bind _returnvalue (Utilities|Time|SetTimerbyEvent (EventDispatchers|CreateEvent :!event Custom|Respawn) (Variables|Default|GetRespawnInterval)))
      (Variables|Default|SetRespawnTimer _returnvalue))))

(event Custom|Respawn
  (Utilities|FlowControl|Sequence
    (:then_0
      ;[0.15 0.15 0.15 0.5] reactivate
      (Variables|Default|SetIsActive true))
    (:then_1
      ;[0.15 0.15 0.15 0.5] Show the Mesh
      (Rendering|SetVisibility (Variables|Default|GetSM_Weapon) true false))
    (:then_2
      ;[0.15 0.15 0.15 0.5] reactivate sphere collision
      (Collision|SetCollisionProfileName (Variables|Default|GetSphere) (Variables|Default|GetActive%20Collision%20Profile) true :!class /Script/Engine.PrimitiveComponent)
      ;[0.15 0.15 0.15 0.5] Play Sound
      (Audio|PlaySoundatLocation (Variables|Default|GetReadySound) (Transformation|GetActorLocation) "0, 0, 0" 1.0 1.0 0.0 0 0 0 0)
      ;[0.15 0.15 0.15 0.5] VFX
      (Niagara|SpawnSystematLocation "/Game/Effects/Particles/Item/NS_GunPad_Pickup_2.NS_GunPad_Pickup_2" (+ (Transformation|GetActorLocation) "0.000000,0.000000,50.000000")))))

(event EventTick
  (params (DeltaSeconds :type Float%20%28single-precision%29))
  (if (Variables|Default|GetIsActive)
    ;[0.15 0.15 0.15 0.5] Rotate the mesh
    (Transformation|AddWorldRotation (Variables|Default|GetSM_Weapon) (Math|Rotator|MakeRotator 0.0 0.0 (* (Variables|Default|GetRotationRate) (Utilities|Time|GetWorldDeltaSeconds))) false false)))

(event EventBeginPlay
  (Collision|AssignOnComponentBeginOverlap (Variables|Default|GetSphere) (delegate Custom|OnComponentBeginOverlap_Event)))

(fn ConstructionScript)